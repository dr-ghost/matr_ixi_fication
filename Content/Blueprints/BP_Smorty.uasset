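; BP_Smorty is the player pawn, with a Glock, a flickering spotlight and health.
; BeginPlay spawns BP_Glock_weapon on the Palm_R socket, and Fire input triggers it, playing an arms montage while ammo remains.
; Damage reduces HealthSmorty, pulsing a vignette through a material parameter collection timeline, or destroys the actor and opens MainMenu at zero.
; Tick uses a gated pair of random delays to toggle the spotlight's flicker light function.
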(event Game|Damage|EventAnyDamage
  (params (Damage :type Float%20%28single-precision%29) (DamageType :type Damage%20Type%20Object%20Reference) (InstigatedBy :type Controller%20Object%20Reference) (DamageCauser :type Actor%20Object%20Reference))
  (Variables|Default|Sethealth_smorty (- (Variables|Default|Gethealth_smorty) Damage))
  (if (<= (Variables|Default|Gethealth_smorty) 0.0)
    (Actor|DestroyActor)
    (Game|OpenLevel(byName) "MainMenu")
    (else
      (bind _float_track (Timeline|vingette PlayFromStart)
        (:Update
          (Rendering|Material|SetScalarParameterValue "/Game/FPWeapon/Materials/Smorty_MPC.Smorty_MPC" "VingetteAmnt" _float_track :!class /Script/Engine.KismetMaterialLibrary))))))

(event EventBeginPlay
  (Variables|Default|Sethealth (Variables|Default|Getmax_health_smorty))
  (bind _returnvalue (Game|SpawnActorfromClass "/Game/Blueprints/BP_Glock_weapon.BP_Glock_weapon_C" (Math|Transform|MakeTransform "0, 0, 0" "0, 0, 0" "1,1,1") "Undefined" 0 0))
  (bind _output_get (Variables|Default|SetPrimaryWeapon _returnvalue))
  (Transformation|AttachComponentToComponent _output_get (Variables|Character|GetMesh) "Palm_R" "KeepRelative" "KeepRelative" "KeepRelative" true))

(event EventTick
  (params (DeltaSeconds :type Float%20%28single-precision%29))
  (if (Variables|Default|GetIsFlickerable)
    (Variables|Default|SetIsFlickerable false)
    (Rendering|Components|Light|SetLightFunctionMaterial (Variables|Default|GetSpotLight) 0)
    (Utilities|FlowControl|Delay (Math|Random|RandomFloatinRange 4.0 7.0))
    (Rendering|Components|Light|SetLightFunctionMaterial (Variables|Default|GetSpotLight) "/Game/Blueprints/Flicker.Flicker")
    (Utilities|FlowControl|Delay (Math|Random|RandomFloatinRange 0.75 2.0))
    (Variables|Default|SetIsFlickerable true)))

(event Input|ActionEvents|InputActionFire
  (params (Key :type Key%20Structure :default "None"))
  (bind _primaryweapon (Variables|Default|GetPrimaryWeapon))
  (:Pressed
    (Default|Fire _primaryweapon)
    (if (> (Variables|/Game/Blueprints/BP_Weapon_base.BP_Weapon_base_C|GetAmmo_ct _primaryweapon) 0)
      (Animation|Montage|PlayMontage (Variables|Character|GetMesh) "/Game/FPWeapon/Weapons/animations/AK_Fire_anim_Skeleton_arms_Montage.AK_Fire_anim_Skeleton_arms_Montage"))))

(fn ConstructionScript)