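; Zombie enemy character that chases the player's BP_Smorty once spotted, attacks it in melee and can be killed.
; PawnSensing triggers an AI MoveTo; on success it plays an attack montage and applies damage, gated by CanAttack until the montage ends.
; HitZombie subtracts health and, at zero, blocks further chasing, plays death montages and disables collision.
; Tick stops movement while the player is unseen; a grunt sound is left unwired.
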(event OnSeePawn(PawnSensing)
  (params (Pawn :type Pawn%20Object%20Reference))
  (Variables|Default|SetisSeeingPlayer1 true)
  (CallFunction|FollowPlayer))

(event Custom|FollowPlayer
  (bind _returnvalue (Game|GetPlayerCharacter 0))
  (bind _asbp_smorty (Utilities|Casting|CastToBP_Smorty _returnvalue))
  (if (and (Variables|Default|GetisSeeingPlayer1) (Variables|Default|Getcanbeattacked))
    (AI|AIMoveTo self "0, 0, 0" _asbp_smorty 5.0 false
      (:then
        (Utilities|FlowControl|Delay 0.5)
        (if (Variables|Default|GetcanAttack)
          (Variables|Default|SetcanAttack false)
          (bind _returnvalue_2 (Animation|PlayAnimMontage "/Game/Animations/zombir_attack.zombir_attack" 1.0 "None"))
          (Game|Damage|ApplyDamage _asbp_smorty (Variables|Default|GetDamage) 0 0)
          (Utilities|FlowControl|Delay _returnvalue_2)
          (Variables|Default|SetcanAttack true))))
    (else
      (Variables|Default|SetisSeeingPlayer1 false))))

(event EventBeginPlay
  (Variables|Default|SetHealth (Variables|Default|GetMax_health)))

(event Collision|EventActorBeginOverlap
  (params (OtherActor :type Actor%20Object%20Reference)))

(event EventTick
  (params (DeltaSeconds :type Float%20%28single-precision%29))
  (if (not (Variables|Default|GetisSeeingPlayer1))
    (Components|Movement|StopMovementImmediately (Variables|Character|GetCharacterMovement))))

(event EventHitZombie
  (params (Damage :type Float%20%28single-precision%29))
  (bind _output_get (Variables|Default|SetHealth (- (Variables|Default|GetHealth) Damage)))
  (if (and (<= _output_get 0.0) (Variables|Default|Getcanbeattacked))
    (Variables|Default|Setcanbeattacked false)
    (Animation|PlayAnimMontage "/Game/Animations/death_montage.death_montage" 1.0 "None")
    (Utilities|FlowControl|Delay 2.0)
    (Variables|Default|Setcanbeattacked false)
    (Collision|SetActorEnableCollision false)
    (Animation|PlayAnimMontage "/Game/Animations/death_zb_montage.death_zb_montage" 1.0 "None")))

(fn ConstructionScript)