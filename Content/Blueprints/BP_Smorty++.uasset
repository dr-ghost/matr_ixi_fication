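; Smorty character Blueprint that handles health, a flickering spotlight, and picking up and dropping items.
; Damage lowers health, destroying the actor at zero or otherwise playing a timeline that drives a vignette through a Material Parameter Collection.
; Tick uses a gated delay loop to toggle the spotlight's flicker light function at random intervals.
; Left Shift attaches an overlapping "pickable" actor to the palm socket; the drop input detaches it onto a downward trace hit.
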(event Game|Damage|EventAnyDamage
  (params (Damage :type Float%20%28single-precision%29) (DamageType :type Damage%20Type%20Object%20Reference) (InstigatedBy :type Controller%20Object%20Reference) (DamageCauser :type Actor%20Object%20Reference))
  (Variables|Default|Sethealth_smorty (- (Variables|Default|Gethealth_smorty) Damage))
  (if (<= (Variables|Default|Gethealth_smorty) 0.0)
    (Actor|DestroyActor)
    (else
      (bind _float_track (Timeline|vingette PlayFromStart)
        (:Update
          (Rendering|Material|SetScalarParameterValue "/Game/FPWeapon/Materials/Smorty_MPC.Smorty_MPC" "VingetteAmnt" _float_track :!class /Script/Engine.KismetMaterialLibrary))))))

(event EventTick
  (params (DeltaSeconds :type Float%20%28single-precision%29))
  (if (Variables|Default|GetIsFlickerable)
    (Variables|Default|SetIsFlickerable false)
    (Rendering|Components|Light|SetLightFunctionMaterial (Variables|Default|GetSpotLight) 0)
    (Utilities|FlowControl|Delay (Math|Random|RandomFloatinRange 4.0 7.0))
    (Rendering|Components|Light|SetLightFunctionMaterial (Variables|Default|GetSpotLight) "/Game/Blueprints/Flicker.Flicker")
    (Utilities|FlowControl|Delay (Math|Random|RandomFloatinRange 0.75 2.0))
    (Variables|Default|SetIsFlickerable true)))

(event Input|ActionEvents|InputActionFire
  (params (Key :type Key%20Structure :default "None")))

(event Input|ActionEvents|InputActiondrop
  (params (Key :type Key%20Structure :default "None"))
  (bind _held_item (Variables|Default|Getheld_item))
  ;[1 1 1] drop item
  (:Pressed
    (if (Variables|Default|GetisHolding)
      (bind (_outhit _returnvalue) (Collision|LineTraceByChannel (Transformation|GetActorLocation) (- (Transformation|GetActorLocation) "0, 0,500.000000") "TraceTypeQuery1" false 0 "None"))
      (if _returnvalue
        (Transformation|DetachFromActor _held_item "KeepWorld" "KeepWorld" "KeepWorld")
        (Transformation|SetActorTransform _held_item (Math|Transform|MakeTransform (.Location (Collision|BreakHitResult _outhit)) "-90.000000, 0, 0" "1,1,1"))
        (Variables|Default|SetisHolding false)))))

(event Input|KeyboardEvents|LeftShift
  (params (Key :type Key%20Structure :default "None"))
  ;[1 1 1] pick up item
  (:Pressed
    (if (not (Variables|Default|GetisHolding))
      (bind _array_element (Utilities|Array|ForEachLoopwithBreak (Collision|GetOverlappingActors "/Script/Matrixification.Knife" :!class /Script/Engine.Actor) :!label _label)
        (:LoopBody
          (if (Actor|ActorHasTag _array_element "pickable")
            (bind _output_get (Variables|Default|Setheld_item _array_element))
            (Transformation|AttachComponentToComponent _output_get (Variables|Character|GetMesh) "Palm_R" "SnapToTarget" "SnapToTarget" "SnapToTarget" true)
            (Variables|Default|SetisHolding true)
            (goto _label Break)))))))

(fn ConstructionScript)