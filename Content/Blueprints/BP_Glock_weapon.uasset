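; Glock weapon Blueprint that fires hitscan shots from the player's camera, or plays a dry-fire sound when empty.
; Firing spends ammo, plays gunshot audio and animation if the player's Cond is set, then line-traces Pawn objects with random spread.
; Hit actors implementing the enemy damage interface receive damage.
; Each shot randomly spawns a tracer actor at the impact point and briefly flashes a muzzle light and mesh, re-randomized afterwards.
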(event EventFire
  (if (> (Variables|Default|GetAmmo_ct) 0)
    (CallFunction|AmmoCheck)
    (bind (_muzzle_loc _impactpoint _hitactor) (CallFunction|LineTrace))
    (if (Utilities|DoesObjectImplementInterface _hitactor "/Game/Blueprints/Enemy_Damage_interface.Enemy_Damage_interface_C")
      (Class|EnemyDamageInterface|HitZombie(Message) _hitactor (Variables|Default|GetDamage)))
    (CallFunction|SpawnDecalTracer _muzzle_loc _impactpoint _impactpoint)
    (Utilities|MuzzleFlsh)
    (else
      (Audio|PlaySoundatLocation "/Game/FPWeapon/Weapons/sounds/DryFire.DryFire" (Transformation|GetWorldLocation (Variables|/Script/Matrixification.Smorty|GetFirstPersonCameraComponent (.AsBP%20Smorty (Utilities|Casting|CastToBP_Smorty (Game|GetPlayerCharacter 0))))) "0, 0, 0" 1.0 1.0 0.0 0 0 0))))

(fn ConstructionScript
  (|CallParentFunction)
  (Variables|Default|SetMax_ammo 20)
  (Variables|Default|SetAmmo_ct 20)
  (Variables|Default|SetBulletSpread 4e+02))

(fn AmmoCheck
  (bind _returnvalue (Math|Random|RandomFloatinRange 0.7 1.2))
  (Math|Integer|DecrementInt (Variables|Default|GetAmmo_ct)
    (:%20%20
      (if (Variables|/Game/Blueprints/BP_Smorty.BP_Smorty_C|Getcond (.AsBP%20Smorty (Utilities|Casting|CastToBP_Smorty (Game|GetPlayerCharacter 0))))
        (Audio|PlaySoundatLocation "/Game/FPWeapon/Weapons/sounds/Gunshot.Gunshot" (Transformation|GetWorldLocation (Variables|/Script/Matrixification.Smorty|GetFirstPersonCameraComponent (.AsBP%20Smorty (Utilities|Casting|CastToBP_Smorty (Game|GetPlayerCharacter 0))))) "0, 0, 0" (+ _returnvalue 2.5) _returnvalue 0.0 0 0 0)
        (Components|Animation|PlayAnimation (Variables|Default|Getweapon) "/Game/FPWeapon/Weapons/animations/AK_Fire_anim_Skeleton_Montage__.AK_Fire_anim_Skeleton_Montage__" false)))))

(fn LineTrace
  (bind _returnvalue (Game|GetPlayerCharacter 0))
  (bind _bulletspread (Variables|Default|GetBulletSpread))
  (bind _muzzle (Variables|Default|Getmuzzle))
  (bind _returnvalue_2 (Transformation|GetWorldLocation _muzzle))
  (bind _returnvalue_3 (* _bulletspread -1.0))
  (bind _asbp_smorty (Utilities|Casting|CastToBP_Smorty _returnvalue))
  (bind _firstpersoncameracomponent (Variables|/Script/Matrixification.Smorty|GetFirstPersonCameraComponent _asbp_smorty))
  (bind _returnvalue_4 (Transformation|GetWorldLocation _firstpersoncameracomponent))
  (bind _outhit (Collision|LineTraceForObjects _returnvalue_4 (+ (+ (* (Math|Vector|GetForwardVector _firstpersoncameracomponent) 2e+04) _returnvalue_4) (Math|Vector|MakeVector (Math|Random|RandomFloatinRange _returnvalue_3 _bulletspread) (Math|Random|RandomFloatinRange _returnvalue_3 _bulletspread) (Math|Random|RandomFloatinRange _returnvalue_3 _bulletspread))) (Utilities|Array|MakeArray "ObjectTypeQuery3") false (Utilities|Array|MakeArray self (.AsBP%20Smorty (Utilities|Casting|CastToBP_Smorty (Game|GetPlayerCharacter 0)))) "None"))
  (bind _outhit_2 (Collision|LineTraceByChannel _returnvalue_2 (.ImpactPoint (Collision|BreakHitResult _outhit)) "TraceTypeQuery1" false 0 "None" true "(R=0.000000,G=0.036052,B=1.000000,A=1.000000)")) ; gun shot
  (return _returnvalue_2 (.ImpactPoint (Collision|BreakHitResult _outhit)) (.HitActor (Collision|BreakHitResult _outhit))))

(fn SpawnDecalTracer
  (params (Location :type Vector) (SpawnTransformLocation :type Vector) (Impact%20Pt :type Vector))
  (if (>= (Math|Random|RandomIntegerinRange 1 10) 5)
    (Game|SpawnActorfromClass "/Game/Blueprints/Tracer_ROund.Tracer_ROund_C" (Math|Transform|MakeTransform SpawnTransformLocation (Transformation|GetWorldRotation (Variables|/Script/Matrixification.Smorty|GetFirstPersonCameraComponent (.AsBP%20Smorty (Utilities|Casting|CastToBP_Smorty (Game|GetPlayerCharacter 0))))) "1.150000,1.150000,1.000000") "Undefined" 0 0))
  (return))